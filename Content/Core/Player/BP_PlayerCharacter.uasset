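; Player character Blueprint that creates and shows the HUD on BeginPlay and routes player input and movement events.
; Two quick slot inputs send a gameplay event tagged for slot selection, with the slot index as payload.
; Landing notifies the movement component a tick later so its state is updated, grapple triggers store state, and E toggles gravity between a forward-axis-based direction and down.
; Disconnected experiments for left-hand IK, mesh attachment, grapple force and health printing remain.
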(event `self.ReceiveTick`
  (params (DeltaSeconds :type "Float (single-precision)")))

(event `self.ReceiveBeginPlay`
  (bind _returnvalue (`|CreateWidget` "/Game/UI/W_HUD.W_HUD_C"))
  (bind _output_get (set `self.HUD` _returnvalue))
  (`UserWidget.AddToViewport` _output_get 0))

(event `EnhancedInput|/Game/Core/Player/Input/Actions/IA_QuickSlot1`
  (params (ActionValue :type Boolean) (ElapsedSeconds :type "Float (double-precision)") (TriggeredSeconds :type "Float (double-precision)") (InputAction :type "InputAction Object Reference" :default "/Game/Core/Player/Input/Actions/IA_QuickSlot1.IA_QuickSlot1"))
  ;[0.03137 0.03137 0.03137] Quick Slots
  (:`Started`
    (`AbilitySystemBlueprintLibrary.SendGameplayEventToActor` self (struct :`TagName` "InputTag.Ability.Quickslot.SelectSlot") (make `GameplayEventData`))))

(event `OnGrappleTrigger`
  (params (bGrappled :type Boolean) (GripPoint :type "Vector Structure"))
  (set `self.Grip Point` GripPoint)
  (set `self.Grappled` bGrappled))

(event `EnhancedInput|/Game/Core/Player/Input/Actions/IA_QuickSlot2`
  (params (ActionValue :type Boolean) (ElapsedSeconds :type "Float (double-precision)") (TriggeredSeconds :type "Float (double-precision)") (InputAction :type "InputAction Object Reference" :default "/Game/Core/Player/Input/Actions/IA_QuickSlot2.IA_QuickSlot2"))
  ;[0.03137 0.03137 0.03137] Quick Slots
  (:`Started`
    (`AbilitySystemBlueprintLibrary.SendGameplayEventToActor` self (struct :`TagName` "InputTag.Ability.Quickslot.SelectSlot") (make `GameplayEventData` :`EventMagnitude` 1.0))))

(event `self.OnLanded`
  (params (Hit :type "HitResult Structure (by ref)"))
  (`KismetSystemLibrary.DelayUntilNextTick`) ; When player lands, the \nMovementComponent\nhas still not been updated
  (`OvrlCharacterMovementComponent.OnPlayerLanded` (`self.GetCharacterMovement`)))

(event `Key|E`
  (params (Key :type "Key Structure"))
  (:`Pressed`
    (`/Engine/EditorBlueprintResources/StandardMacros.FlipFlop`
      (:`A`
        (`CharacterMovementComponent.SetGravityDirection` (`self.CharacterMovement`) (`KismetMathLibrary.NegateVector` (`KismetMathLibrary.Vector_Forward`))))
      (:`B`
        (`CharacterMovementComponent.SetGravityDirection` (`self.CharacterMovement`) (`KismetMathLibrary.Vector_Down`))))))

(fn `UserConstructionScript`)