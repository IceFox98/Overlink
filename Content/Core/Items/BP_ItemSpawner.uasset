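; BP_ItemSpawner is a world item pickup that grants one copy of an item to an overlapping pawn, then destroys itself.
; The construction script sets the mesh and scale from the assigned ItemPickupDefinition when it is valid.
; On PickupCollider overlap, it adds that definition's ItemDefinition to the pawn's InventoryComponent; actors without one, or non-pawns, leave it in place.
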(event `self.PickupCollider.OnComponentBeginOverlap`
  (params (OverlappedComponent :type "PrimitiveComponent Object Reference") (OtherActor :type "Actor Object Reference") (OtherComp :type "PrimitiveComponent Object Reference") (OtherBodyIndex :type Integer) (bFromSweep :type Boolean) (SweepResult :type "HitResult Structure (by ref)"))
  (bind _aspawn (cast `Pawn` OtherActor))
  (bind _returnvalue (`self.GetComponentByClass` _aspawn "/Script/OneBulletMan.InventoryComponent"))
  (`/Engine/EditorBlueprintResources/StandardMacros.IsValid` _returnvalue
    (:`Is Valid`
      (`InventoryComponent.AddItemDefinition` _returnvalue (`PickupDefinition.ItemDefinition` (`self.ItemPickupDefinition`)) 1)
      (`self.K2_DestroyActor`))))

(fn `UserConstructionScript`
  (bind _itemmesh (`self.ItemMesh`))
  (`/Engine/EditorBlueprintResources/StandardMacros.IsValid` (`self.ItemPickupDefinition`)
    (:`Is Valid`
      (`StaticMeshComponent.SetStaticMesh` _itemmesh (`PickupDefinition.DisplayMesh` (`self.ItemPickupDefinition`)))
      (`SceneComponent.SetRelativeScale3D` _itemmesh (`PickupDefinition.MeshScale` (`self.ItemPickupDefinition`))))))