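; GA_Crouch is a Gameplay Ability that toggles the player character between crouched and standing.
; On activation it commits, casts the owning actor to BP_PlayerCharacter, and calls Crouch or UnCrouch based on IsCrouched.
; It notifies the character's ParkourComponent of the new crouch state, then ends immediately, also ending if the commit or cast fails.
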(event `self.K2_ActivateAbility`
  (bind _returnvalue (`self.K2_CommitAbility`))
  (if _returnvalue
    (bind _asbp_player_character (cast `/Game/Core/Player/BP_PlayerCharacter` (`self.GetOwningActorFromActorInfo`))
      (:`then`
        (if (`Character.bIsCrouched` _asbp_player_character)
          (`Character.UnCrouch` _asbp_player_character)
          (bind _parkourcomponent (`PlayerCharacter.ParkourComponent` _asbp_player_character))
          (`ParkourComponent.OnPlayerCrouchChanged` _parkourcomponent false)
          (else
            (`Character.Crouch` _asbp_player_character)
            (`ParkourComponent.OnPlayerCrouchChanged` _parkourcomponent true)))
        (`self.K2_EndAbility`))
      (:`CastFailed`
        (`self.K2_EndAbility` :!label _label)))
    (else
      (goto _label))))