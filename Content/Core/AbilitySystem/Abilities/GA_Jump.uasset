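; GA_Jump is a Gameplay Ability that makes the player character jump.
; After committing, it checks whether the BP_PlayerCharacter is crouched and, if so, activates abilities by the InputTag.Crouch tag.
; It then waits one tick so the movement component can update the crouch state, calls Jump and ends the ability immediately.
; A failed commit or cast just ends the ability.
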(event `self.K2_ActivateAbility`
  (bind _returnvalue (`self.K2_CommitAbility`))
  (if _returnvalue
    (bind _asbp_player_character (cast `/Game/Core/Player/BP_PlayerCharacter` (`self.GetOwningActorFromActorInfo`))
      (:`then`
        (if (`Character.bIsCrouched` _asbp_player_character)
          (`AbilitySystemComponent.TryActivateAbilitiesByTag` (`self.GetAbilitySystemComponentFromActorInfo`) (`BlueprintGameplayTagLibrary.MakeLiteralGameplayTagContainer` (struct :`GameplayTags` (struct :`(TagName` "InputTag.Crouch")))) true))
        (`KismetSystemLibrary.DelayUntilNextTick`) ; This allows MovementComponent to\nactually perform the player crouch.
        (`Character.Jump` _asbp_player_character)
        (`self.K2_EndAbility`))
      (:`CastFailed`
        (`self.K2_EndAbility` :!label _label)))
    (else
      (goto _label))))