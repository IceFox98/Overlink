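; Gameplay ability that reloads the weapon instance passed as the ability's source object.
; It calls StartReloading, then ends at once unless the weapon is still reloading.
; For delayed, animation-driven reloads it waits for the Ovrl.Weapon.ReloadCompleted gameplay event, then calls PerformReload and ends.
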(event `self.K2_ActivateAbility`
  (bind _asovrl_weapon_instance (cast `OvrlWeaponInstance` (`self.GetCurrentSourceObject`))
    (:`then`
      (bind _output_get (set `self.WeaponInstance` _asovrl_weapon_instance))
      (`OvrlWeaponInstance.StartReloading` _output_get)
      (if (`OvrlWeaponInstance.IsReloading` (`self.WeaponInstance`))
        (`AbilityTask_WaitGameplayEvent.WaitGameplayEvent` (struct :`TagName` "Ovrl.Weapon.ReloadCompleted") null ; Wait for delayed reload (animation)
          (:`EventReceived`
            (`OvrlWeaponInstance.PerformReload` (`self.WeaponInstance`))
            (`self.K2_EndAbility`)))
        (else
          (`self.K2_EndAbility`))))
    (:`CastFailed`
      (`self.K2_EndAbility`))))