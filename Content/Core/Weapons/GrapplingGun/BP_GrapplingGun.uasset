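; BP_GrapplingGun is a grappling gun weapon that finds a grip point for the player to grapple onto.
; Its Fire event runs a debug-drawn Visibility line trace from the gun's location along the player's control rotation.
; On a blocking hit, it passes the impact point to BP_PlayerCharacter through OnGrappleTrigger, leaving the grapple response to the character.
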(event `self.Fire`
  (bind _returnvalue (`self.K2_GetActorLocation`))
  (bind _outhit (`KismetSystemLibrary.LineTraceSingle` :`Start` _returnvalue :`End` (+ _returnvalue (* (`KismetMathLibrary.Conv_RotatorToVector` (`Pawn.GetControlRotation` (`GameplayStatics.GetPlayerCharacter` 0))) 5000.0)) :`TraceChannel` "TraceTypeQuery1" :`DrawDebugType` "ForDuration"))
  (bind (_bblockinghit _binitialoverlap _time _distance _location _impactpoint) (`GameplayStatics.BreakHitResult` _outhit))
  (if _bblockinghit
    (bind _asbp_player_character (cast `/Game/Core/Player/BP_PlayerCharacter` (`GameplayStatics.GetPlayerCharacter` 0)))
    (`/Game/Core/Player/BP_PlayerCharacter.OnGrappleTrigger` _asbp_player_character true _impactpoint)))

(fn `UserConstructionScript`)