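; Gameplay ability that fires a projectile weapon.
; On activation it commits, then casts its source object to ProjectileWeapon, ending immediately if that fails.
; It spawns the projectile at the muzzle location, aimed along player 0's camera rotation, passing the damage GameplayEffect and the weapon's instigator.
; It then calls the weapon's Fire and ends.
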(event `self.K2_ActivateAbility`
  (`self.K2_CommitAbility`)
  (bind _asprojectile_weapon (cast `ProjectileWeapon` (`self.GetCurrentSourceObject`))
    (:`then`
      (bind _returnvalue_location (`KismetMathLibrary.BreakTransform` (`ProjectileWeapon.GetMuzzleTransform` _asprojectile_weapon)))
      (`|SpawnActorFromClass` (`self.ProjectileClass`) (`KismetMathLibrary.MakeTransform` _returnvalue_location (`PlayerCameraManager.GetCameraRotation` (`PlayerController.PlayerCameraManager` (`GameplayStatics.GetPlayerController` 0)))) "Undefined" "MultiplyWithRoot" null (`self.GE_Damage`) (`Actor.GetInstigator` _asprojectile_weapon))
      (`WeaponInstance.Fire` _asprojectile_weapon)
      (`self.K2_EndAbility`))
    (:`CastFailed`
      (`self.K2_EndAbility`))))