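; BP_GrabberTool is a weapon-style tool that picks up and drops physics objects through a Physics Handle.
; Firing toggles between grabbing the hit component at its actor's location and releasing the held one, while Tick moves the handle target to GrabbedObjectSlot.
; Held objects use CCD and ignore Pawn collision; release disables CCD, restores Pawn blocking and clamps velocity to limit flinging.
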(event `self.K2_OnFire`
  (params (HitData :type "HitResult Structure (by ref)"))
  (bind (_bblockinghit _binitialoverlap _time _distance _location _impactpoint _normal _impactnormal _physmat _hitactor _hitcomponent) (`GameplayStatics.BreakHitResult` HitData))
  (bind _returnvalue (`PhysicsHandleComponent.GetGrabbedComponent` (`self.PhysicsHandle`)))
  (`/Engine/EditorBlueprintResources/StandardMacros.IsValid` _returnvalue
    (:`Is Valid`
      (`PrimitiveComponent.SetAllUseCCD` _returnvalue false)
      (bind _returnvalue_2 (`PrimitiveComponent.GetPhysicsLinearVelocity` _returnvalue "None"))
      (`PrimitiveComponent.SetAllPhysicsLinearVelocity` _returnvalue (`KismetMathLibrary.Vector_ClampSizeMax` _returnvalue_2 2000.0) false)
      (`PrimitiveComponent.SetCollisionResponseToChannel` _returnvalue "ECC_Pawn" "ECR_Block")
      (`PhysicsHandleComponent.ReleaseComponent` (`self.PhysicsHandle`)))
    (:`Is Not Valid`
      (`PrimitiveComponent.SetCollisionResponseToChannel` _hitcomponent "ECC_Pawn" "ECR_Ignore")
      (`PhysicsHandleComponent.GrabComponentAtLocation` (`self.PhysicsHandle`) _hitcomponent "None" (`self.K2_GetActorLocation` _hitactor))
      (`PrimitiveComponent.SetAllUseCCD` _hitcomponent true))))

(event `self.ReceiveTick`
  (params (DeltaSeconds :type "Float (single-precision)"))
  (`/Engine/EditorBlueprintResources/StandardMacros.IsValid` (`PhysicsHandleComponent.GetGrabbedComponent` (`self.PhysicsHandle`))
    (:`Is Valid`
      (`PhysicsHandleComponent.SetTargetLocation` (`self.PhysicsHandle`) (`SceneComponent.K2_GetComponentLocation` (`self.GrabbedObjectSlot`))))))

(fn `UserConstructionScript`)